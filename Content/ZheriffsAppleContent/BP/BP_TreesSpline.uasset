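; Spline-placed row of dead trees that spawns apples during play.
; The construction script adds tree meshes at regular spacing along the spline with random yaw and scale, giving roughly a quarter of them a glowing material.
; A looping timer checks the world's apple count against the Zheriff game state's minimum, and when at or below it spawns an apple at a random socket on a random tree, skipping colliding spots.
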(event `self.ReceiveBeginPlay`
  (`|ExecutionSequence`
    (:`then_0`
      (bind _asbp_zheriff_game_state (cast `/Game/ZheriffsAppleContent/Core/BP_ZheriffGameState` (`GameplayStatics.GetGameState`)))
      (set `self.AppleGameState` _asbp_zheriff_game_state))
    (:`then_1`
      (`KismetSystemLibrary.K2_SetTimer` null "SpawnApples" 3.0 true))))

(fn `SpawnApples`
  (locals (SelectedTree :type "StaticMeshComponent Object Reference"))
  (bind _trees (`self.Trees`))
  (bind _outactors (`GameplayStatics.GetAllActorsOfClass` "/Game/ZheriffsAppleContent/BP/BP_Apple.BP_Apple_C"))
  (if (<= (`KismetArrayLibrary.Array_Length` _outactors) (`/Game/ZheriffsAppleContent/Core/BP_ZheriffGameState.AppleCountMin` (`self.AppleGameState`)))
    (bind _output_get (set `local.SelectedTree` (`|GetArrayItem` _trees (`KismetMathLibrary.RandomInteger` (`KismetArrayLibrary.Array_Length` _trees)))))
    (`/Engine/EditorBlueprintResources/StandardMacros.IsValid` _output_get
      (:`Is Valid`
        (bind _returnvalue (`SceneComponent.GetAllSocketNames` _output_get))
        (`|SpawnActorFromClass` "/Game/ZheriffsAppleContent/BP/BP_Apple.BP_Apple_C" (`KismetMathLibrary.MakeTransform` (`SceneComponent.GetSocketLocation` _output_get (`|GetArrayItem` _returnvalue (`KismetMathLibrary.RandomInteger` (`KismetArrayLibrary.Array_Length` _returnvalue))))) "DontSpawnIfColliding" "OverrideRootScale" null null)))))

(fn `UserConstructionScript`
  (bind (_returnvalue_roll _returnvalue_pitch _returnvalue_yaw) (`KismetMathLibrary.BreakRotator` (`KismetMathLibrary.RandomRotator` false)))
  (for _index (range (+ (/ (`KismetMathLibrary.Round` (`SplineComponent.GetSplineLength` (`self.Spline`))) (`self.SpaceBetween`)) 1))
    (bind _returnvalue (`AddComponent|NODE_AddStaticMeshComponent-0` :`RelativeTransform` (`KismetMathLibrary.MakeTransform` (`SplineComponent.GetLocationAtDistanceAlongSpline` (`self.Spline`) (`KismetMathLibrary.Conv_IntToDouble` (* _index (`self.SpaceBetween`))) "Local") (`KismetMathLibrary.MakeRotator` 0.0 0.0 _returnvalue_yaw) (* (1.0 1.0 1.0) (`KismetMathLibrary.RandomFloatInRange` 0.8 1.2)))))
    (`StaticMeshComponent.SetStaticMesh` _returnvalue (`self.TreeMesh`))
    (`KismetArrayLibrary.Array_Add` (`self.Trees`) _returnvalue)
    (if (>= (`KismetMathLibrary.RandomInteger` 100) 75)
      (`PrimitiveComponent.SetMaterial` _returnvalue 0 "/Game/ZheriffsAppleContent/Visualization/Materials/M_DeadTree_Glow.M_DeadTree_Glow")
      (else
        (`PrimitiveComponent.SetMaterial` _returnvalue 0 "/Game/ZheriffsAppleContent/Visualization/Materials/M_DeadTree.M_DeadTree")))))