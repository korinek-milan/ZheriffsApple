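; Saloon interactable that serves as the apple-paid exit ending the game, priced by the game state's apple count.
; EnableLights opens it, turning on its point light and igniting two child-actor campfires.
; While the action is held, a looping timer moves one collected apple into the payment every half second and updates the HUD.
; Once the price is paid it calls EndGame on the caller; partial payments persist between holds.
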(event `self.ReceiveBeginPlay`
  (set `self.Price` (`/Game/ZheriffsAppleContent/Core/BP_ZheriffGameState.AppleCountToUnlockEnd` (cast `/Game/ZheriffsAppleContent/Core/BP_ZheriffGameState` (`GameplayStatics.GetGameState`) :!pure true))))

(event `EnableLights`
  (`|ExecutionSequence`
    (:`then_0`
      (`SceneComponent.SetVisibility` (`self.PointLight`) true false))
    (:`then_1`
      (bind _asbp_campfire (cast `/Game/ZheriffsAppleContent/BP/BP_Campfire` (`ChildActorComponent.ChildActor` (`self.BP_Campfire`))))
      (`/Game/ZheriffsAppleContent/BP/BP_Campfire.Ignite` _asbp_campfire))
    (:`then_2`
      (bind _asbp_campfire_2 (cast `/Game/ZheriffsAppleContent/BP/BP_Campfire` (`ChildActorComponent.ChildActor` (`self.BP_Campfire2`))))
      (`/Game/ZheriffsAppleContent/BP/BP_Campfire.Ignite` _asbp_campfire_2))
    (:`then_3`
      (set `self.bOpen` true))))

(event `self.StartAction`
  (params (Caller :type "/Game/ZheriffsAppleContent/Characters/Player/BP_FirstPersonCharacter Object Reference"))
  (if (`self.bOpen`)
    (bind _output_get (set `self.Caller` Caller))
    (set `self.HUD` (`/Game/ZheriffsAppleContent/Characters/Player/BP_FirstPersonCharacter.HUD` _output_get))
    (set `self.bActionRunning` true)
    (bind _returnvalue (`KismetSystemLibrary.K2_SetTimer` null "CheckPickupTime" 0.1 true))
    (set `self.PickupTimer` _returnvalue)
    (set `self.ActionTimeStart` (`GameplayStatics.GetTimeSeconds`))))

(event `self.StopAction`
  (params (Caller :type "/Game/ZheriffsAppleContent/Characters/Player/BP_FirstPersonCharacter Object Reference"))
  (set `self.bActionRunning` false))

(event `CheckPickupTime`
  (bind _caller (`self.Caller`))
  (if (and (`self.bActionRunning`) (> (`/Game/ZheriffsAppleContent/Characters/Player/BP_FirstPersonCharacter.CollectedApples` (`self.Caller`)) 0))
    (if (>= (- (`GameplayStatics.GetTimeSeconds`) (`self.ActionTimeStart`)) 0.5)
      (set `self.ActionTimeStart` (`GameplayStatics.GetTimeSeconds`))
      (`/Engine/EditorBlueprintResources/StandardMacros.IncrementInt` (`self.AllreadyPaid`)
        (:`  `
          (`/Engine/EditorBlueprintResources/StandardMacros.DecrementInt` (`/Game/ZheriffsAppleContent/Characters/Player/BP_FirstPersonCharacter.CollectedApples` _caller)
            (:`  `
              (`/Game/ZheriffsAppleContent/Characters/Player/BP_FirstPersonCharacter.AppleNoise` _caller false))))))
    (`/Game/ZheriffsAppleContent/HUD/BP_HUD.SetProgressPercent` (`self.HUD`) (/ (`self.AllreadyPaid`) (`self.Price`)))
    (`/Game/ZheriffsAppleContent/HUD/BP_HUD.SetScoreText` (`self.HUD`) (`/Game/ZheriffsAppleContent/Characters/Player/BP_FirstPersonCharacter.CollectedApples` (`self.Caller`)))
    (bind _text (`self.GetInteractiveText`))
    (`/Game/ZheriffsAppleContent/HUD/BP_HUD.ShowHideActionWidget` (`self.HUD`) true _text)
    (if (>= (`self.AllreadyPaid`) (`self.Price`))
      (set `self.bActionRunning` false)
      (`/Game/ZheriffsAppleContent/Characters/Player/BP_FirstPersonCharacter.EndGame` (`self.Caller`) "NewEnumerator1"))
    (else
      (`KismetSystemLibrary.K2_ClearAndInvalidateTimerHandle` (`self.PickupTimer`)))))

(fn `GetInteractiveText`
  (returns (Text :type Text))
  (if (`self.bOpen`)
    (return (`KismetTextLibrary.Conv_StringToText` (`KismetStringLibrary.Concat_StrStr` "Hold E - Pay for a ticket to the Kingdom Come \n" (`KismetStringLibrary.Conv_IntToString` (- (`self.Price`) (`self.AllreadyPaid`))) " Apples left")))
    (else
      (return ""))))

(fn `HasHoldAction`
  (returns (bHoldAction :type Boolean))
  (return true))

(fn `UserConstructionScript`)