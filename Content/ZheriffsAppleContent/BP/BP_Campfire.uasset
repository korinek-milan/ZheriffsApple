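; BP_Campfire is an interactable campfire that the player lights with a torch, counting toward a game-ending condition.
; Interaction ignites it only when the caller's torch is visible and the fire is out, turning on its point light and particles.
; Light visibility serves as the lit state; once every campfire is lit, ignition calls EndGame on the player character.
; Optional auto-extinguish puts it out on a timer.
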(event `Ignite`
  (`SceneComponent.SetVisibility` (`self.PointLight`) true false)
  (`ActorComponent.Activate` (`self.ParticleSystem`) true)
  (bind _ballignes (`self.CheckAllIgnites`))
  (if _ballignes
    (`/Game/ZheriffsAppleContent/Characters/Player/BP_FirstPersonCharacter.EndGame` (cast `/Game/ZheriffsAppleContent/Characters/Player/BP_FirstPersonCharacter` (`GameplayStatics.GetPlayerCharacter` 0) :!pure true) "NewEnumerator3"))
  (if (`self.bAutoExtinguish`)
    (`KismetSystemLibrary.K2_SetTimer` null "Extinguish" 30.0)))

(event `Extinguish`
  (`SceneComponent.SetVisibility` (`self.PointLight`) false false)
  (`ActorComponent.Deactivate` (`self.ParticleSystem`)))

(event `/Game/ZheriffsAppleContent/BP/BPI_Interactive.StartAction`
  (params (Caller :type "/Game/ZheriffsAppleContent/Characters/Player/BP_FirstPersonCharacter Object Reference"))
  (if (and (`SceneComponent.IsVisible` (`/Game/ZheriffsAppleContent/Characters/Player/BP_FirstPersonCharacter.Torch` Caller)) (not (`SceneComponent.bVisible` (`self.PointLight`))))
    (`self.Ignite`)))

(fn `CheckAllIgnites`
  (returns (bAllIgnes :type Boolean))
  (bind _outactors (`GameplayStatics.GetAllActorsOfClass` "BP_Campfire_C"))
  (for _array_element _outactors
    (if (not (`SceneComponent.bVisible` (`/Game/ZheriffsAppleContent/BP/BP_Campfire.PointLight` _array_element)))
      (return false)))
  (return true))

(fn `GetInteractiveText`
  (returns (Text :type Text))
  (return (select `bool` (`SceneComponent.bVisible` (`self.PointLight`)) :`false` "E - Ignite with a torch" :!type "Text")))

(fn `HasHoldAction`
  (returns (bHoldAction :type Boolean))
  (return false))

(fn `UserConstructionScript`)