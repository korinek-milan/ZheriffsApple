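; BP_Item is an interactable shop item that players buy with collected apples for a movement or pickup upgrade.
; When the action starts, it checks the caller's apple count against Price, deducts the cost, notifies the caller of the ItemType bought and destroys itself.
; Its interaction prompt builds text from ItemType and Price, and it reports no hold action, so purchase is a single press.
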(event `/Game/ZheriffsAppleContent/BP/BPI_Interactive.StartAction`
  (params (Caller :type "/Game/ZheriffsAppleContent/Characters/Player/BP_FirstPersonCharacter Object Reference"))
  (bind _collectedapples (`/Game/ZheriffsAppleContent/Characters/Player/BP_FirstPersonCharacter.CollectedApples` Caller))
  (bind _price (`self.Price`))
  (if (>= _collectedapples _price)
    (set `/Game/ZheriffsAppleContent/Characters/Player/BP_FirstPersonCharacter.CollectedApples` (- _collectedapples _price) Caller)
    (`/Game/ZheriffsAppleContent/Characters/Player/BP_FirstPersonCharacter.ItemBought` Caller (`self.ItemType`))
    (`self.K2_DestroyActor`)))

(fn `getInteractiveText`
  (returns (Text :type Text))
  (return (`KismetTextLibrary.Conv_StringToText` (`KismetStringLibrary.Concat_StrStr` "Press E to buy - " (select `/Game/ZheriffsAppleContent/BP/EItem` (`self.ItemType`) :`NewEnumerator0` "Faster movement" :`NewEnumerator1` "Faster pickup") " \n" (`KismetStringLibrary.Conv_IntToString` (`self.Price`)) " Apples"))))

(fn `hasHoldAction`
  (returns (bHoldAction :type Boolean))
  (return false))

(fn `UserConstructionScript`)