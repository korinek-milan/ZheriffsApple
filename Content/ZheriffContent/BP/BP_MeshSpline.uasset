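; BP_MeshSpline is a construction-time placement tool that lines copies of a tree mesh along a spline.
; Its construction script appends the SplinePoints array to the spline in local space, then adds a static mesh component at regular SpaceBetween distance intervals along its length.
; Each new component receives TreeMesh and is stored in the Trees array, and the existing Tree01 component gets the same mesh.
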(fn `UserConstructionScript`
  (`StaticMeshComponent.SetStaticMesh` (`self.Tree01`) (`self.TreeMesh`))
  (for _array_element (`self.SplinePoints`)
    (`SplineComponent.AddSplinePoint` (`self.Spline`) _array_element "Local" true))
  (for _index (range (+ (/ (`KismetMathLibrary.Round` (`SplineComponent.GetSplineLength` (`self.Spline`))) (`self.SpaceBetween`)) 1))
    (bind _returnvalue (`AddComponent|NODE_AddStaticMeshComponent-0` :`RelativeTransform` (`KismetMathLibrary.MakeTransform` (`SplineComponent.GetLocationAtDistanceAlongSpline` (`self.Spline`) (`KismetMathLibrary.Conv_IntToDouble` (* _index (`self.SpaceBetween`))) "Local") (`self.Relative Transform Rotation`))))
    (`StaticMeshComponent.SetStaticMesh` _returnvalue (`self.TreeMesh`))
    (`KismetArrayLibrary.Array_Add` (`self.Trees`) _returnvalue)))