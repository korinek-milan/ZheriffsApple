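; BP_Apple is an interactive apple pickup that the player collects by holding E.
; StartAction takes the pickup time and HUD from the caller, then runs a looping timer that updates the progress bar until completion or StopAction interrupts it.
; Success notifies the caller; either outcome tints a dynamic material green or red, animates its emissive strength by timeline, then destroys the apple, so interrupted pickups are also lost.
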(event `Collected/Failed`
  (params (bCollected :type Boolean))
  (bind _materialinstance (`self.MaterialInstance`))
  ;[1 1 1] Change color before destroy - green success, red failed
  (if bCollected
    (`MaterialInstanceDynamic.SetVectorParameterValue` _materialinstance "Color" (struct :`G` 1.0 :`A` 1.0))
    (bind (_direction _emissivestrength) (`Timeline|Timeline_0` :!label _label)
      (:`Update`
        (`MaterialInstanceDynamic.SetScalarParameterValue` (`self.MaterialInstance`) "EmissiveStrength" _emissivestrength))
      (:`Finished`
        (`KismetSystemLibrary.Delay` 0.5)
        (`self.K2_DestroyActor`)))
    (else
      (`MaterialInstanceDynamic.SetVectorParameterValue` _materialinstance "Color" (struct :`R` 1.0 :`A` 1.0))
      (goto _label))))

(event `/Game/ZheriffContent/BP/BPI_Interactive.StartAction`
  (params (Caller :type "/Game/ZheriffContent/Characters/Player/BP_FirstPersonCharacter Object Reference"))
  (set `self.Caller` Caller)
  (set `self.HUD` (`/Game/ZheriffContent/Characters/Player/BP_FirstPersonCharacter.HUD` Caller))
  (set `self.Pickup Time` (`/Game/ZheriffContent/Characters/Player/BP_FirstPersonCharacter.PickupTime` Caller))
  (set `self.PickupTimeStart` (`GameplayStatics.GetTimeSeconds`))
  (set `self.bActionRunning` true)
  ;[1 1 1] Timer executes event for checking hold button and update loading bar
  (bind _returnvalue (`KismetSystemLibrary.K2_SetTimer` null "CheckPickupTime" 0.1 true))
  (set `self.PickupTimer` _returnvalue))

(event `/Game/ZheriffContent/BP/BPI_Interactive.StopAction`
  (params (Caller :type "/Game/ZheriffContent/Characters/Player/BP_FirstPersonCharacter Object Reference"))
  (set `self.bActionRunning` false))

(event `CheckPickupTime`
  (bind _returnvalue (- (`GameplayStatics.GetTimeSeconds`) (`self.PickupTimeStart`)))
  (if (`self.bActionRunning`)
    ;[1 1 1] Successfully collected
    (if (>= _returnvalue (`self.Pickup Time`))
      (`KismetSystemLibrary.K2_ClearAndInvalidateTimerHandle` (`self.PickupTimer`))
      (`self.Collected/Failed` true)
      (`/Game/ZheriffContent/Characters/Player/BP_FirstPersonCharacter.AppleCollected` (`self.Caller`))
      (else
        ;[1 1 1] Collection in progress - update loading bar
        (`/Game/ZheriffContent/HUD/BP_HUD.SetProgressPercent` (`self.HUD`) (/ _returnvalue (`self.Pickup Time`)))))
    (else
      ;[1 1 1] Collecting was interrupted
      (`KismetSystemLibrary.K2_ClearAndInvalidateTimerHandle` (`self.PickupTimer`))
      (`self.Collected/Failed` false))))

(fn `getInteractiveText`
  (returns (Text :type Text))
  (return "Hold E - Pickup"))

(fn `hasHoldAction`
  (returns (bHoldAction :type Boolean))
  (return true))

(fn `UserConstructionScript`
  (bind _returnvalue (`KismetMaterialLibrary.CreateDynamicMaterialInstance` "/Game/ZheriffContent/Visualization/Materials/M_Apple.M_Apple"))
  (bind _output_get (set `self.MaterialInstance` _returnvalue))
  (`PrimitiveComponent.SetMaterial` (`self.AppleSM`) 0 _output_get))