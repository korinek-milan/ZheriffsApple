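; AI controller for zombies that runs the BT_Zombie behavior tree and feeds its blackboard.
; On BeginPlay it seeds the blackboard with the first BP_PatrollingPoints actor found, walk and run speeds, and an initial zombie state.
; AI perception updates involving the first-person character write whether the player is sensed and their location, using the stimulus location or, while sensed, the player's current position.
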(event `self.ReceiveBeginPlay`
  (bind _returnvalue (`AIBlueprintHelperLibrary.GetBlackboard` null))
  (`self.RunBehaviorTree` "/Game/ZheriffContent/AI/BT_Zombie.BT_Zombie")
  (`|ExecutionSequence`
    (:`then_0`
      (bind _outactors (`GameplayStatics.GetAllActorsOfClass` "/Game/ZheriffContent/BP/BP_PatrollingPoints.BP_PatrollingPoints_C"))
      (`BlackboardComponent.SetValueAsObject` (`AIBlueprintHelperLibrary.GetBlackboard` null) "PatrolPathObject" (`|GetArrayItem` _outactors)))
    (:`then_1`
      (`BlackboardComponent.SetValueAsFloat` _returnvalue "WalkSpeed" 150.0)
      (`BlackboardComponent.SetValueAsFloat` _returnvalue "RunSpeed" 400.0))
    (:`then_2`
      (`BlackboardComponent.SetValueAsEnum` (`AIBlueprintHelperLibrary.GetBlackboard` null) "ZombieState" (enumliteral `/Game/ZheriffContent/AI/EZombieState` "NewEnumerator0")))))

(event `self.AIPerception.OnTargetPerceptionUpdated`
  (params (Actor :type "Actor Object Reference") (Stimulus :type "AIStimulus Structure"))
  (bind (_age _expirationage _strength _stimuluslocation _receiverlocation _tag _bsuccessfullysensed) (break `AIStimulus` Stimulus))
  (bind _returnvalue (`AIBlueprintHelperLibrary.GetBlackboard` null))
  (cast `/Game/ZheriffContent/Characters/Player/BP_FirstPersonCharacter` Actor)
  (`BlackboardComponent.SetValueAsBool` _returnvalue "bSeePlayer" _bsuccessfullysensed)
  (`BlackboardComponent.SetValueAsVector` _returnvalue "PlayerLocation" _stimuluslocation)
  (if _bsuccessfullysensed
    (`BlackboardComponent.SetValueAsVector` (`AIBlueprintHelperLibrary.GetBlackboard` null) "PlayerLocation" (`self.K2_GetActorLocation` (`GameplayStatics.GetPlayerCharacter` 0)))))

(fn `UserConstructionScript`)